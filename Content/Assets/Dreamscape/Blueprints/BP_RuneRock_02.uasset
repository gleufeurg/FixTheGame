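; BP_RuneRock_02 is a rune stone that activates when struck by a thrown BP_Potion.
; On activation it swaps its main and emissive textures through a dynamic material instance, then checks the activation state of the linked Runes, handling both RuneRock_01 and RuneRock_02 types.
; A separate Invoc event plays a sound and spawns a BP_Phoenix with an assigned Path; the rune check shown does not call it.
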(event `self.ReceiveHit`
  (params (MyComp :type "PrimitiveComponent Object Reference") (Other :type "Actor Object Reference") (OtherComp :type "PrimitiveComponent Object Reference") (bSelfMoved :type Boolean) (HitLocation :type "Vector Structure") (HitNormal :type "Vector Structure") (NormalImpulse :type "Vector Structure") (Hit :type "HitResult Structure (by ref)"))
  (bind _asbp_potion (cast `/Game/Assets/Dreamscape/Blueprints/BP_Potion` Other))
  (if (`/Game/Assets/Dreamscape/Blueprints/BP_Potion.isThrow` _asbp_potion)
    (bind _returnvalue (`PrimitiveComponent.CreateDynamicMaterialInstance` (`self.StaticMeshComponent`) 0 "/Game/Assets/Dreamscape/Materials/Rocks/MI_RuneRock_01.MI_RuneRock_01" "None"))
    (`MaterialInstanceDynamic.SetTextureParameterValue` _returnvalue "Main Texture" "/Game/Assets/Dreamscape/Textures/Rocks/T_RuneRock_02_C_NEWN.T_RuneRock_02_C_NEWN")
    (`MaterialInstanceDynamic.SetTextureParameterValue` _returnvalue "Emissive" "/Game/Assets/Dreamscape/Textures/Rocks/T_RuneRock_02_E_NEWN.T_RuneRock_02_E_NEWN")
    (set `self.bIsActivate` true)
    (for _array_element (`self.Runes`)
      (bind _asbp_rune_rock_01 (cast `/Game/Assets/Dreamscape/Blueprints/BP_RuneRock_01` _array_element)
        (:`then`
          (if (not (`/Game/Assets/Dreamscape/Blueprints/BP_RuneRock_01.bIsActivate` _asbp_rune_rock_01))
            (break)))
        (:`CastFailed`
          (bind _asbp_rune_rock_02 (cast `/Game/Assets/Dreamscape/Blueprints/BP_RuneRock_02` _array_element))
          (if (not (`/Game/Assets/Dreamscape/Blueprints/BP_RuneRock_02.bIsActivate` _asbp_rune_rock_02))
            (break)))))
    (bind _asbp_rune_rock_01_2 (cast `/Game/Assets/Dreamscape/Blueprints/BP_RuneRock_01` _array_element)
      (:`then`
        (if (`/Game/Assets/Dreamscape/Blueprints/BP_RuneRock_01.bIsActivate` _asbp_rune_rock_01_2)
          _))
      (:`CastFailed`
        (bind _asbp_rune_rock_02_2 (cast `/Game/Assets/Dreamscape/Blueprints/BP_RuneRock_02` _array_element))
        (if (`/Game/Assets/Dreamscape/Blueprints/BP_RuneRock_02.bIsActivate` _asbp_rune_rock_02_2)
          _)))))

(event `Invoc`
  (bind _spawn_transform_location (`KismetMathLibrary.BreakTransform` (`self.Spawn Transform`)))
  (`GameplayStatics.PlaySoundAtLocation` "/Game/Assets/Sounds/WeirdSound.WeirdSound" _spawn_transform_location (struct) 1.0 1.0 0.0 null null null null)
  (bind _returnvalue (`|SpawnActorFromClass` "/Game/Assets/Dreamscape/Mobs/phoenix-bird/source/BP_Phoenix.BP_Phoenix_C" (`self.Spawn Transform`) "Undefined" "OverrideRootScale" null null))
  (set `/Game/Assets/Dreamscape/Mobs/phoenix-bird/source/BP_Phoenix.Path` (`self.Path`) _returnvalue))

(fn `UserConstructionScript`)