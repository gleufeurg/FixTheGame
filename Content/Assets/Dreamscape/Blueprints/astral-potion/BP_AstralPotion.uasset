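; BP_AstralPotion is an astral potion bottle actor that serves as a pickup or, when flagged IsThrow, a thrown breakable.
; Non-thrown potions spawn an ambient Niagara effect shortly after BeginPlay and remove it when destroyed.
; Overlapping BP_CustomTPS grants Number potions through GainAstralPotion and destroys the actor, with no IsThrow check.
; On a hit, thrown potions spawn an explosion effect, play a glass-break sound and destroy themselves.
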(event `self.ReceiveDestroyed`
  (if (not (`self.isThrow`))
    (`ActorComponent.K2_DestroyComponent` (stale `self.ReceiveBeginPlay` _returnvalue))))

(event `self.ReceiveBeginPlay`
  (bind _sm_bottle (`self.SM_bottle`))
  (`KismetSystemLibrary.Delay` 0.02)
  (if (not (`self.isThrow`))
    (bind _returnvalue (`NiagaraFunctionLibrary.SpawnSystemAtLocation` "/Game/Assets/Effects/Particle_Systems/NS_PotionAmbient.NS_PotionAmbient" (`SceneComponent.K2_GetComponentLocation` _sm_bottle) (`SceneComponent.K2_GetComponentRotation` _sm_bottle)))))

(event `self.Collision.OnComponentBeginOverlap`
  (params (OverlappedComponent :type "PrimitiveComponent Object Reference") (OtherActor :type "Actor Object Reference") (OtherComp :type "PrimitiveComponent Object Reference") (OtherBodyIndex :type Integer) (bFromSweep :type Boolean) (SweepResult :type "HitResult Structure (by ref)"))
  (bind _asbp_custom_tps (cast `/Game/Blueprints/BP_CustomTPS` OtherActor))
  (`/Game/Blueprints/BP_CustomTPS.GainAstralPotion` _asbp_custom_tps (`self.Number`))
  (`self.K2_DestroyActor`))

(event `self.ReceiveHit`
  (params (MyComp :type "PrimitiveComponent Object Reference") (Other :type "Actor Object Reference") (OtherComp :type "PrimitiveComponent Object Reference") (bSelfMoved :type Boolean) (HitLocation :type "Vector Structure") (HitNormal :type "Vector Structure") (NormalImpulse :type "Vector Structure") (Hit :type "HitResult Structure (by ref)"))
  (if (`self.isThrow`)
    (`self.Destroy`)))

(event `Destroy`
  (bind _sm_bottle (`self.SM_bottle`))
  (`NiagaraFunctionLibrary.SpawnSystemAtLocation` "/Game/Assets/Effects/Particle_Systems/NS_PotionExplode.NS_PotionExplode" (`SceneComponent.K2_GetComponentLocation` _sm_bottle) (`SceneComponent.K2_GetComponentRotation` _sm_bottle))
  (`GameplayStatics.PlaySoundAtLocation` "/Game/Assets/Sounds/glass-break.glass-break" (`self.K2_GetActorLocation`) (struct) 1.0 1.0 0.0 null null null null)
  (`self.K2_DestroyActor`))

(fn `UserConstructionScript`)