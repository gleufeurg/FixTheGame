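; BP_Potion_01 is a potion bottle actor that can be picked up by the player or shatter when thrown.
; On BeginPlay it spawns an ambient Niagara effect at the bottle mesh's position, without attaching it.
; Overlap with BP_CustomTPS calls GainPotion with its Number and destroys the actor.
; On hit, if IsThrow is set, it spawns an explosion effect and destroys itself, with no damage logic.
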(event `self.ReceiveBeginPlay`
  (bind _sm_bottle (`self.SM_bottle`))
  (`NiagaraFunctionLibrary.SpawnSystemAtLocation` "/Game/Assets/Effects/Particle_Systems/NS_PotionAmbient.NS_PotionAmbient" (`SceneComponent.K2_GetComponentLocation` _sm_bottle) (`SceneComponent.K2_GetComponentRotation` _sm_bottle)))

(event `self.ReceiveActorBeginOverlap`
  (params (OtherActor :type "Actor Object Reference"))
  (bind _asbp_custom_tps (cast `/Game/Blueprints/BP_CustomTPS` OtherActor))
  (`/Game/Blueprints/BP_CustomTPS.gainPotion` _asbp_custom_tps (`self.Number`))
  (`self.K2_DestroyActor`))

(event `self.ReceiveHit`
  (params (MyComp :type "PrimitiveComponent Object Reference") (Other :type "Actor Object Reference") (OtherComp :type "PrimitiveComponent Object Reference") (bSelfMoved :type Boolean) (HitLocation :type "Vector Structure") (HitNormal :type "Vector Structure") (NormalImpulse :type "Vector Structure") (Hit :type "HitResult Structure (by ref)"))
  (bind _sm_bottle (`self.SM_bottle`))
  (if (`self.isThrow`)
    (`NiagaraFunctionLibrary.SpawnSystemAtLocation` "/Game/Assets/Effects/Particle_Systems/NS_PotionExplode.NS_PotionExplode" (`SceneComponent.K2_GetComponentLocation` _sm_bottle) (`SceneComponent.K2_GetComponentRotation` _sm_bottle))
    (`self.K2_DestroyActor`)))

(fn `UserConstructionScript`)