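; Phoenix bird mob that flies along a spline path and can be caught with a thrown astral potion.
; At BeginPlay it starts its Path, then on Tick, throttled by a short Delay, copies the transform of the path's RefPoints.
; At the spline's end it resets the distance, destroying itself unless the path loops.
; A thrown potion overlap sends CaptureMessage to BP_CustomTPS, plays a sound and destroys both actors.
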(event `self.ReceiveBeginPlay`
  (bind _path (`self.Path`))
  (`KismetSystemLibrary.Delay` 0.01)
  (if (not (== _path null))
    (set `/Game/Assets/Dreamscape/Mobs/phoenix-bird/BP_Path.start` true _path)))

(event `self.ReceiveActorBeginOverlap`
  (params (OtherActor :type "Actor Object Reference"))
  (bind _asbp_astral_potion (cast `/Game/Assets/Dreamscape/Blueprints/astral-potion/BP_AstralPotion` OtherActor))
  (if (`/Game/Assets/Dreamscape/Blueprints/astral-potion/BP_AstralPotion.isThrow` _asbp_astral_potion)
    (bind _outactors (`GameplayStatics.GetAllActorsOfClass` "/Game/Blueprints/BP_CustomTPS.BP_CustomTPS_C"))
    (message `/Game/Blueprints/I_Capture.Capture` _outactors (`self.Number`))
    (`/Game/Assets/Dreamscape/Blueprints/astral-potion/BP_AstralPotion.Destroy` _asbp_astral_potion)
    (`GameplayStatics.PlaySoundAtLocation` "/Game/Assets/Sounds/SFXCaught.SFXCaught" (`self.K2_GetActorLocation`) (struct) 1.0 1.0 0.0 null null null null)
    (`self.K2_DestroyActor`)))

(event `self.ReceiveTick`
  (params (DeltaSeconds :type "Float (single-precision)"))
  (bind _path (`self.Path`))
  (bind (_returnvalue_location _returnvalue_rotation) (`KismetMathLibrary.BreakTransform` (`SceneComponent.K2_GetComponentToWorld` (`/Game/Assets/Dreamscape/Mobs/phoenix-bird/BP_Path.RefPoints` _path))))
  ;[0.3281 0.3281 0.3281] Follow spline
  (if (not (== _path null))
    (`KismetSystemLibrary.Delay` 0.02)
    (`self.K2_SetActorTransform` (`KismetMathLibrary.MakeTransform` _returnvalue_location _returnvalue_rotation))
    (if (> (`/Game/Assets/Dreamscape/Mobs/phoenix-bird/BP_Path.Distance` _path) (`SplineComponent.GetSplineLength` (`/Game/Assets/Dreamscape/Mobs/phoenix-bird/BP_Path.Spline` _path)))
      (if (`/Game/Assets/Dreamscape/Mobs/phoenix-bird/BP_Path.bIsLooping` _path)
        (set `/Game/Assets/Dreamscape/Mobs/phoenix-bird/BP_Path.Distance` 0.0 _path)
        (else
          (set `/Game/Assets/Dreamscape/Mobs/phoenix-bird/BP_Path.Distance` 0.0 _path)
          (`self.K2_DestroyActor`))))))

(fn `UserConstructionScript`)